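; BP_Desk is an actor whose Box trigger decides the game's outcome from the stone that overlaps it.
; On BeginPlay it registers itself with GoGameMode and passes it a restart callback.
; A BP_BlackStone overlap shows the win widget and a BP_WhiteStone shows the failure widget.
; Either result disables Box collision to block further triggers, and the restart callback restores it to query-only.
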(event `self.ReceiveBeginPlay`
  (bind _asgo_game_mode (cast `GoGameMode` (`GameplayStatics.GetGameMode`)))
  (`GoGameMode.SetDesk` _asgo_game_mode self)
  (add `GoGameMode.OnRestart` _asgo_game_mode (delegate `OnRestart_Event`)))

(event `OnRestart_Event`
  (`PrimitiveComponent.SetCollisionEnabled` (`self.Box`) "QueryOnly"))

(event `self.ReceiveActorBeginOverlap`
  (params (OtherActor :type "Actor Object Reference")))

(event `self.Box.OnComponentBeginOverlap`
  (params (OverlappedComponent :type "PrimitiveComponent Object Reference") (OtherActor :type "Actor Object Reference") (OtherComp :type "PrimitiveComponent Object Reference") (OtherBodyIndex :type Integer) (bFromSweep :type Boolean) (SweepResult :type "HitResult Structure (by ref)"))
  (cast `/Game/Actors/BP_BlackStone` OtherActor
    (:`then`
      (bind _returnvalue (`|CreateWidget` "/Game/UI/WBP_Win.WBP_Win_C"))
      (`UserWidget.AddToViewport` _returnvalue 0)
      (`PrimitiveComponent.SetCollisionEnabled` (`self.Box`) "NoCollision"))
    (:`CastFailed`
      (cast `/Game/Actors/BP_WhiteStone` OtherActor)
      (bind _returnvalue_2 (`|CreateWidget` "/Game/UI/WBP_Failed.WBP_Failed_C"))
      (`UserWidget.AddToViewport` _returnvalue_2 0)
      (`PrimitiveComponent.SetCollisionEnabled` (`self.Box`) "NoCollision"))))

(fn `UserConstructionScript`)